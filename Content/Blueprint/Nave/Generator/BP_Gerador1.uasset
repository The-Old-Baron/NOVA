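; Ship generator actor that spins four rotor meshes each Tick and tracks temperature driven by torque.
; SpeedGraphicReturn spools rotors up sequentially through chained timelines at increasing multipliers, while SetGeneration raises their speeds instantly.
; SetTorque adjusts temperature, which recolors the beam particles, turning red at critical, and prints a debug readout.
; Torque never reaches rotor speed, and consumption, catalyst, water, fuel, pressure and friction setters are empty stubs.
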(event EventSpeedGraphicReturn
  (params (Speed :type Float%20%28double-precision%29))
  (if (not (<= Speed 0.0))
    (bind _delta (Timeline|SpeedAccressed PlayFromStart)
      (:Update
        (Variables|Grafico|SetRotator%20Speed%201 (Math|Float|Lerp (Variables|Grafico|GetRotator%20Speed%201) Speed _delta)))
      (:Finished
        (bind _delta_2 (Timeline|Timeline PlayFromStart)
          (:Update
            (Variables|Grafico|SetRotator%20Speed%202 (Math|Float|Lerp (Variables|Grafico|GetRotator%20Speed%202) (* Speed 1.3) _delta_2)))
          (:Finished
            (bind _delta_3 (Timeline|Timeline_0 PlayFromStart)
              (:Update
                (Variables|Grafico|SetRotator%20Speed%203 (Math|Float|Lerp (Variables|Grafico|GetRotator%20Speed%203) (* Speed 1.6) _delta_3)))
              (:Finished
                (bind _delta_4 (Timeline|Timeline_1 PlayFromStart)
                  (:Update
                    (Variables|Grafico|SetRotator%20Speed%204 (Math|Float|Lerp (Variables|Grafico|GetRotator%20Speed%204) (* Speed 2.0) _delta_4))
                    (Variables|Atrito|SetCur_Atrito (Math|Float|Lerp Speed (Variables|Atrito|GetMax_Atrito) 0.0))))))))))))

(event EventSetTorque
  (params (NewTorque :type Float%20%28double-precision%29))
  (CallFunction|UpdateTorque NewTorque))

(event EventTick
  (params (DeltaSeconds :type Float%20%28single-precision%29))
  ;[1 1 1] Movement
  (Transformation|AddLocalRotation (Variables|Default|GetGasDynamicTrap1_part1_1) (Math|Rotator|MakeRotator (Variables|Grafico|GetRotator%20Speed%201) 0.0 0.0) false false)
  (Transformation|AddLocalRotation (Variables|Default|GetGasDynamicTrap1_part1_2) (Math|Rotator|MakeRotator (Variables|Grafico|GetRotator%20Speed%202) 0.0 0.0) false false)
  (Transformation|AddLocalRotation (Variables|Default|GetGasDynamicTrap1_part1_3) (Math|Rotator|MakeRotator (Variables|Grafico|GetRotator%20Speed%203) 0.0 0.0) false false)
  (Transformation|AddLocalRotation (Variables|Default|GetGasDynamicTrap1_part2) (Math|Rotator|MakeRotator (Variables|Grafico|GetRotator%20Speed%204) 0.0 0.0) false false))

(fn ConstructionScript
  ;[1 1 1] Material
  (Rendering|Material|SetMaterial (Variables|Default|GetGasDynamicTrap) 0 (Variables|Grafico|GetMaterial)))

(fn SetGeneration
  (params (Potencia :type Float%20%28double-precision%29))
  (if (not (<= Potencia 0.0))
    (while (>= Potencia (Variables|Grafico|GetRotator%20Speed%201))
      (Variables|Grafico|SetRotator%20Speed%201 (+ (Variables|Grafico|GetRotator%20Speed%201) 0.1)))
    (while (>= (* (Variables|Grafico|GetRotator%20Speed%201) 1.1) (Variables|Grafico|GetRotator%20Speed%202))
      (Variables|Grafico|SetRotator%20Speed%202 (+ (Variables|Grafico|GetRotator%20Speed%202) 0.1)))
    (while (>= (* (Variables|Grafico|GetRotator%20Speed%202) 1.3) (Variables|Grafico|GetRotator%20Speed%203))
      (Variables|Grafico|SetRotator%20Speed%203 (+ (Variables|Grafico|GetRotator%20Speed%203) 0.1)))
    (while (>= (* (Variables|Grafico|GetRotator%20Speed%203) 1.5) (Variables|Grafico|GetRotator%20Speed%204))
      (Variables|Grafico|SetRotator%20Speed%204 (+ (Variables|Grafico|GetRotator%20Speed%204) 0.1)))))

(fn UpdateTorque
  (params (NewTorque :type Float%20%28double-precision%29))
  (if (> NewTorque (Variables|Torque|GetCur_Torque))
    (bind _output_get (Variables|Torque|SetCur_Torque NewTorque))
    (CallFunction|SetTemperatura (+ (* _output_get 0.3) (Variables|Temperatura|GetCur_Temperatura)))
    (else
      (bind _output_get_2 (Variables|Torque|SetCur_Torque NewTorque))
      (CallFunction|SetTemperatura (- (Variables|Temperatura|GetCur_Temperatura) (* _output_get_2 0.3))))))

(fn SetConsumo
  (params (SetConsumo :type Float%20%28double-precision%29)))

(fn SetCatalizador
  (params (SetCatalizador :type Float%20%28double-precision%29)))

(fn SetAgua
  (params (Agua :type Float%20%28double-precision%29)))

(fn SetCombustivel
  (params (Combustivel :type Float%20%28double-precision%29)))

(fn SetTemperatura
  (params (Temperatura :type Float%20%28double-precision%29))
  (bind _hsv (Class|KismetMathLibrary|RGBtoHSVVector "(R=1.000000,G=0.000000,B=0.042986,A=1.000000)"))
  (bind _returnvalue (* Temperatura 1e+02))
  (bind _ps_beam2 (Variables|Default|GetPS_Beam2))
  (bind _max_temperatura (Variables|Temperatura|GetMax_Temperatura))
  (bind _ps_beam2_2 (Variables|Default|GetPS_Beam2))
  (bind _returnvalue_2 (/ _returnvalue _max_temperatura))
  (bind _returnvalue_3 (/ _returnvalue_2 1e+02))
  (bind _returnvalue_4 (Math|Conversions|ToLinearColor(Float) _returnvalue_3))
  (if (>= Temperatura (Variables|Temperatura|GetTemperaturaCritica))
    (Effects|Components|ParticleSystem|SetColorParameter _ps_beam2 "BeamColor1" _hsv)
    (Effects|Components|ParticleSystem|SetColorParameter _ps_beam2 "BeamColor2" _hsv)
    (Effects|Components|ParticleSystem|SetColorParameter _ps_beam2 "BeamColor3" _hsv)
    (Effects|Components|ParticleSystem|SetColorParameter _ps_beam2 "BeamColor4" _hsv)
    (Effects|Components|ParticleSystem|SetColorParameter _ps_beam2 "BeamColor5" _hsv)
    (Effects|Components|ParticleSystem|SetColorParameter _ps_beam2 "BeamColor6" _hsv)
    (Effects|Components|ParticleSystem|SetColorParameter _ps_beam2 "BeamColor7" _hsv)
    (else
      (Effects|Components|ParticleSystem|SetColorParameter _ps_beam2_2 "BeamColor1" _returnvalue_4)
      (Effects|Components|ParticleSystem|SetColorParameter _ps_beam2_2 "BeamColor2" _returnvalue_4)
      (Effects|Components|ParticleSystem|SetColorParameter _ps_beam2_2 "BeamColor3" _returnvalue_4)
      (Effects|Components|ParticleSystem|SetColorParameter _ps_beam2_2 "BeamColor4" _returnvalue_4)
      (Effects|Components|ParticleSystem|SetColorParameter _ps_beam2_2 "BeamColor5" _returnvalue_4)
      (Effects|Components|ParticleSystem|SetColorParameter _ps_beam2_2 "BeamColor6" _returnvalue_4)
      (Effects|Components|ParticleSystem|SetColorParameter _ps_beam2_2 "BeamColor7" _returnvalue_4)))
  (bind _output_get (Variables|Temperatura|SetCur_Temperatura Temperatura))
  (Rendering|Debug|DrawDebugString "-3810.000000,960.000000,-550.000000" (Utilities|String|ToString(Text) (Utilities|Text|FormatText "Temperatura: {Value}" _output_get)) 0 "(R=1.000000,G=1.000000,B=1.000000,A=1.000000)" 0.1))

(fn SetPressao
  (params (Pressao :type Float%20%28double-precision%29)))

(fn SetAtrito
  (params (Atrito :type Float%20%28double-precision%29)))

(fn GetTemperatura
  (return (Variables|Temperatura|GetCur_Temperatura) (Variables|Temperatura|GetMax_Temperatura) (Variables|Temperatura|GetMin_Temperatura) (Variables|Temperatura|GetTemperaturaCritica)))