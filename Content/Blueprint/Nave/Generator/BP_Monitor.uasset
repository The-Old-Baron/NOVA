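; BP_Monitor is an interactable monitor on the ship that opens a generator control UI for the player.
; On BeginPlay it searches actors implementing BPI_Gerador and stores the one matching its Tag as Reator.
; Interacting creates WBP_GeneratorController bound to that generator, adds it to the viewport and shows the mouse cursor.
; The fracture, item type and mesh getters return only fixed or empty values.
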(event EventInteractwith
  (bind _returnvalue (Game|GetPlayerController 0))
  (bind _returnvalue_2 (UserInterface|CreateWidget "/Game/Blueprint/Nave/WBP_GeneratorController.WBP_GeneratorController_C" _returnvalue (Variables|Default|GetReator)))
  (UserInterface|Viewport|AddtoViewport _returnvalue_2 0)
  (Variables|/Script/Engine.PlayerController|SetbShowMouseCursor _returnvalue true)
  (Class|WidgetBlueprintLibrary|SetFocustoGameViewport))

(event EventBeginPlay
  (bind _outactors (Actor|GetAllActorswithInterface "/Game/Blueprint/Nave/Generator/BPI_Gerador.BPI_Gerador_C"))
  (for _array_element _outactors
    (if (Actor|ActorHasTag _array_element (Variables|Default|GetTag))
      (Variables|Default|SetReator _array_element))))

(fn ConstructionScript)

(fn GetFractureBool
  (return false))

(fn GetItemType
  (return "NewEnumerator0"))

(fn GetMesh
  (return 0))