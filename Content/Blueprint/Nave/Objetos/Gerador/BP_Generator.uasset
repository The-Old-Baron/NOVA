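; Ship generator actor that converts torque and catalyst into energy while running, tracking temperature, coolant and durability.
; Delay-gated Tick computes output, resets and recalculates temperature, wears durability when critical, and refreshes text readouts; rotors spin every frame.
; Positive SetTorque recolors the beam, adjusts BPI_NaveStatus actors' reducer energy by subtracting then re-adding output, and ramps four rotors through chained Timelines.
; Setters and getters expose generator state.
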(event EventTick
  (params (DeltaSeconds :type Float%20%28single-precision%29))
  (bind _temperature_max (Variables|Temperature|GetTemperature_Max))
  (bind _temperature_min (Variables|Temperature|GetTemperature_Min))
  (Utilities|FlowControl|Sequence
    (:then_0
      (Utilities|FlowControl|Delay 0.2)
      (CallFunction|UpdateText)
      (if (Math|Boolean|ORBoolean (<= (Variables|Fuel|GetFuel_Cur) 0.0) (<= (Variables|Misc|GetDurability) 0.0) (not (Variables|Misc|GetIsOn)) (<= (Variables|Misc|GetTorque) 1e+01))
        (if (>= (Variables|Temperature|GetTemperature_Cur) 0.0)
          (Variables|Temperature|SetTemperature_Cur (- (Variables|Temperature|GetTemperature_Cur) (* 1.0 DeltaSeconds)))
          (Variables|Graphic|SetRotator%20Speed%201 0.0)
          (Variables|Graphic|SetRotator%20Speed%202 0.0)
          (Variables|Graphic|SetRotator%20Speed%203 0.0)
          (Variables|Graphic|SetRotator%20Speed%204 0.0))
        (else
          (bind _returnvalue (CallFunction|CalcGeneration DeltaSeconds))
          (Variables|Misc|SetEnergyOutput _returnvalue)
          (bind _output_get (Variables|Temperature|SetTemperature_Consumption (- (* (Variables|Misc|GetTorque) 5.0) (* (Variables|Coolant|GetCoolant_Consumption) 2.5))))
          (Variables|Temperature|SetTemperature_Cur 0.0)
          (bind _output_get_2 (Variables|Temperature|SetTemperature_Cur (+ (* _output_get DeltaSeconds) (Variables|Temperature|GetTemperature_Cur))))
          (if (<= _output_get_2 _temperature_min)
            (Variables|Temperature|SetTemperature_Cur _temperature_min)
            (elif (>= _output_get_2 _temperature_max)
              (Variables|Temperature|SetTemperature_Cur _temperature_max)))
          (if (>= (Variables|Temperature|GetTemperature_Cur) (Variables|Temperature|GetTemperature_Critical))
            (Variables|Misc|SetDurability (- (Variables|Misc|GetDurability) (* (Variables|Temperature|GetTemperature_Cur) DeltaSeconds))))
          (Variables|Coolant|SetCoolant_Cur (- (Variables|Coolant|GetCoolant_Cur) (* DeltaSeconds (* 0.5 (Variables|Coolant|GetCoolant_Consumption)))))
          (if (<= (Variables|Misc|GetDurability) 0.0)
            (Variables|Misc|SetIsOn false)))))
    (:then_1
      ;[1 1 1] Movement
      (Transformation|AddLocalRotation (Variables|Default|GetGasDynamicTrap1_part1_1) (Math|Rotator|MakeRotator (Variables|Graphic|GetRotator%20Speed%201) 0.0 0.0) false false)
      (Transformation|AddLocalRotation (Variables|Default|GetGasDynamicTrap1_part1_2) (Math|Rotator|MakeRotator (Variables|Graphic|GetRotator%20Speed%202) 0.0 0.0) false false)
      (Transformation|AddLocalRotation (Variables|Default|GetGasDynamicTrap1_part1_3) (Math|Rotator|MakeRotator (Variables|Graphic|GetRotator%20Speed%203) 0.0 0.0) false false)
      (Transformation|AddLocalRotation (Variables|Default|GetGasDynamicTrap1_part2) (Math|Rotator|MakeRotator (Variables|Graphic|GetRotator%20Speed%204) 0.0 0.0) false false))))

(event EventSetTorque
  (params (NewTorque :type Float%20%28double-precision%29))
  (bind _energyoutput (Variables|Misc|GetEnergyOutput))
  (bind _output_get (Variables|Misc|SetTorque NewTorque))
  (if (not (<= _output_get 0.0))
    (CallFunction|GraphicUpdate)
    (bind _outactors (Actor|GetAllActorswithInterface "/Game/Blueprint/Nave/BPI_NaveStatus.BPI_NaveStatus_C"))
    (for _array_element _outactors
      (bind _reducer (Class|BPINaveStatus|GetEnergyReducer(Message) _array_element))
      (Class|BPINaveStatus|SetReducerEnergy(Message) _array_element (- _reducer _energyoutput))
      (bind _reducer_2 (Class|BPINaveStatus|GetEnergyReducer(Message) _array_element))
      (Class|BPINaveStatus|SetReducerEnergy(Message) _array_element (- _reducer_2 (* _energyoutput -1.0)))
      (bind _value (Timeline|Timeline PlayFromStart)
        (:Update
          (Variables|Graphic|SetRotator%20Speed%201 (Math|Float|Lerp (Variables|Graphic|GetRotator%20Speed%201) (/ _output_get 1e+03) _value)))
        (:Finished
          (bind _value_2 (Timeline|Timeline_3 PlayFromStart)
            (:Update
              (Variables|Graphic|SetRotator%20Speed%202 (Math|Float|Lerp (Variables|Graphic|GetRotator%20Speed%202) (* (/ _output_get 1e+03) 1.3) _value_2)))
            (:Finished
              (bind _value_3 (Timeline|Timeline_0 PlayFromStart)
                (:Update
                  (Variables|Graphic|SetRotator%20Speed%203 (Math|Float|Lerp (Variables|Graphic|GetRotator%20Speed%203) (* (/ _output_get 1e+03) 1.6) _value_3)))
                (:Finished
                  (bind _value_4 (Timeline|Timeline_1 PlayFromStart)
                    (:Update
                      (Variables|Graphic|SetRotator%20Speed%204 (Math|Float|Lerp (Variables|Graphic|GetRotator%20Speed%204) (* (/ _output_get 1e+03) 2.0) _value_4)))))))))))))

(event EventSetCatalizator
  (params (NewCatalizator :type Float%20%28double-precision%29))
  (Variables|Catalizator|SetCatalizator_Consumption NewCatalizator))

(event EventSetCoolant
  (params (NewCoolant :type Float%20%28double-precision%29))
  (Variables|Coolant|SetCoolant_Consumption NewCoolant))

(event EventTurn
  (Variables|Misc|SetIsOn (not (Variables|Misc|GetIsOn))))

(event EventSpeedGraphicReturn
  (params (New%20Speed :type Float%20%28double-precision%29)))

(fn ConstructionScript
  ;[1 1 1] Material
  (Rendering|Material|SetMaterial (Variables|Default|GetGasDynamicTrap) 0 (Variables|Default|GetMaterial)))

(fn SetGeneration
  (params (Potencia :type Float%20%28double-precision%29))
  (if (<= Potencia 0.0)
    (Variables|Graphic|SetRotator%20Speed%201 0.0)
    (Variables|Graphic|SetRotator%20Speed%202 0.0)
    (Variables|Graphic|SetRotator%20Speed%203 0.0)
    (Variables|Graphic|SetRotator%20Speed%204 0.0)
    (else
      (while (>= Potencia (Variables|Graphic|GetRotator%20Speed%201))
        (Variables|Graphic|SetRotator%20Speed%201 (+ (Variables|Graphic|GetRotator%20Speed%201) 0.1)))
      (while (>= (* (Variables|Graphic|GetRotator%20Speed%201) 1.1) (Variables|Graphic|GetRotator%20Speed%202))
        (Variables|Graphic|SetRotator%20Speed%202 (+ (Variables|Graphic|GetRotator%20Speed%202) 0.1)))
      (while (>= (* (Variables|Graphic|GetRotator%20Speed%202) 1.3) (Variables|Graphic|GetRotator%20Speed%203))
        (Variables|Graphic|SetRotator%20Speed%203 (+ (Variables|Graphic|GetRotator%20Speed%203) 0.1)))
      (while (>= (* (Variables|Graphic|GetRotator%20Speed%203) 1.5) (Variables|Graphic|GetRotator%20Speed%204))
        (Variables|Graphic|SetRotator%20Speed%204 (+ (Variables|Graphic|GetRotator%20Speed%204) 0.1))))))

(fn ReactorAnimation
  (CallFunction|SetGeneration (Variables|Misc|GetTorque))
  (Transformation|AddLocalRotation (Variables|Default|GetGasDynamicTrap1_part1_1) (Math|Rotator|MakeRotator (Variables|Graphic|GetRotator%20Speed%201) 0.0 0.0) false false)
  (Transformation|AddLocalRotation (Variables|Default|GetGasDynamicTrap1_part1_2) (Math|Rotator|MakeRotator (Variables|Graphic|GetRotator%20Speed%202) 0.0 0.0) false false)
  (Transformation|AddLocalRotation (Variables|Default|GetGasDynamicTrap1_part1_3) (Math|Rotator|MakeRotator (Variables|Graphic|GetRotator%20Speed%203) 0.0 0.0) false false)
  (Transformation|AddLocalRotation (Variables|Default|GetGasDynamicTrap1_part2) (Math|Rotator|MakeRotator (Variables|Graphic|GetRotator%20Speed%204) 0.0 0.0) false false))

(fn UpdateText
  (Rendering|Components|TextRender|SetText (Variables|Default|Gettxt_Temperatura) (Utilities|Text|FormatText "Temperatura: {value} °C" (Variables|Temperature|GetTemperature_Cur)))
  (Rendering|Components|TextRender|SetText (Variables|Default|Gettxt_EnergyOut) (Utilities|Text|FormatText "{value} kW/J" (Variables|Misc|GetEnergyOutput)))
  (Rendering|Components|TextRender|SetText (Variables|Default|Gettxt_Durabilidade) (Utilities|Text|FormatText "{value} %" (Variables|Misc|GetDurability)))
  (Rendering|Components|TextRender|SetText (Variables|Default|Gettxt_Torque) (Utilities|Text|FormatText "{Value} N*m" (Variables|Misc|GetTorque))))

(fn GraphicUpdate
  (bind _ps_beam2 (Variables|Default|GetPS_Beam2))
  (bind _temperature_cur (Variables|Temperature|GetTemperature_Cur))
  (bind _returnvalue (Math|Float|Clamp(Float) _temperature_cur))
  (bind _returnvalue_2 (Math|Color|MakeColor 1.0 0.0 0.0 _returnvalue))
  (bind _returnvalue_3 (* "(R=1.000000,G=0.000000,B=0.091064,A=1.000000)" _returnvalue_2))
  (bind _returnvalue_4 (Class|KismetMathLibrary|RGBLineartoHSV _returnvalue_3))
  (if (>= _temperature_cur 0.0)
    (Effects|Components|ParticleSystem|SetColorParameter _ps_beam2 "BeamColor1" _returnvalue_4)
    (Effects|Components|ParticleSystem|SetColorParameter _ps_beam2 "BeamColor2" _returnvalue_4)
    (Effects|Components|ParticleSystem|SetColorParameter _ps_beam2 "BeamColor3" _returnvalue_4)
    (Effects|Components|ParticleSystem|SetColorParameter _ps_beam2 "BeamColor4" _returnvalue_4)))

(fn CalcGeneration
  (params (B :type Float%20%28double-precision%29))
  (return (* (* (/ (Variables|Misc|GetTorque) 1e+02) (Variables|Catalizator|GetCatalizator_Cur)) B)))

(fn GetCatalizator
  (return (Variables|Catalizator|GetCatalizator_Consumption) (Variables|Catalizator|GetCatalizator_Cur) (Variables|Catalizator|GetCatalizator%20Min) (Variables|Catalizator|GetCatalizator%20Max)))

(fn GetCoolant
  (return (Variables|Coolant|GetCoolant_Cur) (Variables|Coolant|GetCoolant_Max) (Variables|Coolant|GetCoolant_Min) (Variables|Coolant|GetCoolant_Consumption)))

(fn GetEnergyGen
  (return (Variables|Misc|GetEnergyOutput)))

(fn GetFuel
  (return (Variables|Fuel|GetFuel_Max) (Variables|Fuel|GetFuel_Cur) (Variables|Fuel|GetFuel_Min) (Variables|Fuel|GetFuel_Consumption)))

(fn GetGeneratorState
  (return (Variables|Misc|GetIsOn)))

(fn GetQuality
  (return (Variables|Misc|GetDurability)))

(fn GetTemperature
  (return (Variables|Temperature|GetTemperature_Cur) (Variables|Temperature|GetTemperature_Max) (Variables|Temperature|GetTemperature_Min) (Variables|Temperature|GetTemperature_Consumption) (Variables|Temperature|GetTemperature_Critical)))