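; BP_Monitor is an interactable ship monitor that opens a generator controller UI for a linked reactor.
; On BeginPlay it searches actors implementing BPI_Gerador and stores the one matching its Tag as Reator.
; Interacting while not InUse creates WBP_GeneratorController with the reactor and monitor, shows the cursor and sets InUse.
; InUseState allows that flag to be set externally; its OnRep handler is empty.
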(event EventInteractwith
  (bind _returnvalue (Game|GetPlayerController 0))
  (if (not (Variables|Default|GetInUse))
    (bind _returnvalue_2 (UserInterface|CreateWidget "/Game/HUD/Nave/WBP_GeneratorController.WBP_GeneratorController_C" _returnvalue (Variables|Default|GetReator) self))
    (UserInterface|Viewport|AddtoViewport _returnvalue_2 0)
    (Variables|/Script/Engine.PlayerController|SetbShowMouseCursor _returnvalue true)
    (Class|WidgetBlueprintLibrary|SetFocustoGameViewport)
    (Variables|Default|SetInUse true)))

(event EventBeginPlay
  (Variables|Default|SetInUse false)
  (bind _outactors (Actor|GetAllActorswithInterface "/Game/Blueprint/Nave/Objetos/Gerador/BPI_Gerador.BPI_Gerador_C"))
  (for _array_element _outactors
    (if (Actor|ActorHasTag _array_element (Variables|Default|GetTag))
      (Variables|Default|SetReator _array_element))))

(fn ConstructionScript)

(fn OnRepinUse)

(fn InUseState
  (params (NewState :type Boolean))
  (Variables|Default|SetInUse NewState))

(fn GetFractureBool
  (return false))

(fn GetItemType
  (return "NewEnumerator0"))

(fn GetMesh
  (return 0))