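; Ship actor that simulates oxygen, energy and fuel (combustivel) drain and reports to a WD_NaveMonitor widget.
; Three looping timelines subtract random amounts up to each reducer, with setters and energy-load events adjusting values.
; Energy and fuel refresh the monitor as they change, while oxygen does so only when out of bounds.
; Depleted energy sends OffMessage to all BPI_Lamp actors; the getters return only zero.
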(event EventSetOxigen
  (params (SetOxigen :type Float%20%28double-precision%29))
  (Variables|Default|SetOxigen SetOxigen))

(event EventSetEnergy
  (params (Energy :type Float%20%28double-precision%29))
  (Variables|Default|SetEnergy Energy))

(event EventSetCombustivelConsumo
  (params (Combustivel :type Float%20%28double-precision%29))
  (Variables|Default|SetCombustivelReducer Combustivel))

(event EventSetCombustivel
  (params (Combustivel :type Float%20%28double-precision%29))
  (Variables|Default|SetCombustivel Combustivel))

(event EventAddEnergyReducer
  (params (AddReducer :type Float%20%28double-precision%29))
  (Variables|Default|SetEnergyReducerFactory (+ AddReducer (Variables|Default|GetEnergyReducerFactory))))

(event EventRemoveEnergyReducer
  (params (RemoveReducer :type Float%20%28double-precision%29))
  (Variables|Default|SetEnergyReducerFactory (- RemoveReducer (Variables|Default|GetEnergyReducerFactory))))

(event EventSetReducerEnergy
  (params (Energy :type Float%20%28double-precision%29))
  (Variables|Default|SetEnergyReducerFactory Energy))

(event EventBeginPlay
  (Utilities|FlowControl|Sequence
    (:then_0
      (Timeline|Timeline_1 Play
        (:Loop
          (CallFunction|OxigenUpdate))))
    (:then_1
      (Timeline|Timeline_3 Play
        (:Loop
          (CallFunction|EnergyUpdate))))
    (:then_2
      (bind _aswd_nave_monitor (Utilities|Casting|CastToWD_NaveMonitor (UserInterface|GetWidget (Variables|Default|GetWidget))))
      (Variables|Default|SetAs%20WD%20Nave%20Monitor _aswd_nave_monitor))
    (:then_3
      (Timeline|Timeline_4 Play
        (:Loop
          (CallFunction|CombustivelUpdate))))))

(fn ConstructionScript)

(fn OxigenUpdate
  (if (or (<= (- (Variables|Default|GetOxigen) (Math|Random|RandomFloatinRange 0.0 (Variables|Default|GetOxigenReducerFactor))) 0.0) (>= (- (Variables|Default|GetOxigen) (Math|Random|RandomFloatinRange 0.0 (Variables|Default|GetOxigenReducerFactor))) (Variables|Default|GetMaxOxigen)))
    (Default|SetOxigen (Variables|Default|GetAs%20WD%20Nave%20Monitor) (stale _output_get) (Variables|Default|GetMaxOxigen))
    (else
      (bind _output_get (Variables|Default|SetOxigen (- (Variables|Default|GetOxigen) (Math|Random|RandomFloatinRange 0.0 (Variables|Default|GetOxigenReducerFactor))))))))

(fn Shutdown
  (bind _outactors (Actor|GetAllActorswithInterface "/Game/Meshes/Rooms/Lamps/BPI_Lamp.BPI_Lamp_C"))
  (for _array_element _outactors
    (Class|BPILamp|Off(Message) _array_element)))

(fn CombustivelUpdate
  (bind _maxcombustivel (Variables|Default|GetMaxCombustivel))
  (if (not (or (<= (- (Variables|Default|GetCombustivel) (Math|Random|RandomFloatinRange 0.0 (Variables|Default|GetCombustivelReducer))) 0.0) (>= (- (Variables|Default|GetCombustivel) (Math|Random|RandomFloatinRange 0.0 (Variables|Default|GetCombustivelReducer))) _maxcombustivel)))
    (bind _output_get (Variables|Default|SetCombustivel (- (Variables|Default|GetCombustivel) (Math|Random|RandomFloatinRange 0.0 (Variables|Default|GetCombustivelReducer)))))
    (Default|SetCombustivel (Variables|Default|GetAs%20WD%20Nave%20Monitor) _output_get _maxcombustivel)))

(fn EnergyUpdate
  (bind _maxenergy (Variables|Default|GetMaxEnergy))
  (if (<= (- (Variables|Default|GetEnergy) (Math|Random|RandomFloatinRange 0.0 (Variables|Default|GetEnergyReducerFactory))) 0.0)
    (CallFunction|Shutdown)
    (elif (not (>= (- (Variables|Default|GetEnergy) (Math|Random|RandomFloatinRange 0.0 (Variables|Default|GetEnergyReducerFactory))) _maxenergy))
      (bind _output_get (Variables|Default|SetEnergy (- (Variables|Default|GetEnergy) (Math|Random|RandomFloatinRange 0.0 (Variables|Default|GetEnergyReducerFactory)))))
      (Default|SetEnergy (Variables|Default|GetAs%20WD%20Nave%20Monitor) _output_get _maxenergy (Variables|Default|GetEnergyReducerFactory)))))

(fn GetCombustivel
  (return 0.0))

(fn GetCombustivelConsumo
  (return 0.0))

(fn GetEnergy
  (return 0.0))

(fn GetEnergyReducer
  (return 0.0))

(fn GetOxigen
  (return 0.0 0.0))

(fn GetOxigenReducer
  (return 0.0))