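; Spline-based wire prop that builds its spline mesh segments in the Construction Script through the Wire function.
; SplineMeshVar selects segment placement: between spline points, or at fixed Spacing along the spline with scaled direction tangents.
; WireVar picks one of six component variants, all scaled by WireSize.
; Each segment gets MI_Wire dynamic instances for colour, dirt, specular, roughness and TextureVar's texture set, with some variants using a second material slot.
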(fn ConstructionScript
  (|Wire))