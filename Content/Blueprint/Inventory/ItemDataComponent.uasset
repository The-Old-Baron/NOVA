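; Item data component that turns its owning actor into a pickup for the player's inventory.
; On BeginPlay it enables replication on the owner.
; Interaction passes the item's data table row name and quantity to the player's InventorySystem, then destroys the owner behind an always-true branch, without checking the add result.
; The LookAt function is a stub that returns empty text.
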(event EventTick
  (params (DeltaSeconds :type Float%20%28single-precision%29)))

(event EventInteractwith
  (params (PlayerCharacter :type BPC%20Player%20Object%20Reference))
  (bind _inventory_system (Variables|/Game/Blueprint/Player/BPC_Player.BPC_Player_C|GetInventory_System PlayerCharacter))
  (Utilities|IsValid _inventory_system
    (:Is%20Valid
      (Default|AddtoInventory _inventory_system (.rowname (Variables|Default|GetItemID)) (Variables|Default|GetQuantity))
      (if true
        (Actor|DestroyActor (Components|GetOwner))))))

(event EventBeginPlay
  (Networking|SetReplicates (Components|GetOwner) true))

(fn Lookat
  (return ""))