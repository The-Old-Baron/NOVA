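; BP_Lamp03 is a lamp that switches on and off and reports its energy cost to the ship (Nave) status system.
; On and Off swap the mesh material and message every actor implementing BPI_NaveStatus with EnergyCost.
; Off calls AddEnergyReducer and On calls RemoveEnergyReducer.
; The construction script calls On, so the lamp starts lit and also sends that message during construction.
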(event EventOff
  (Rendering|Material|SetMaterial (Variables|Default|GetSM_Lamp04) 0 (Variables|Default|GetMaterial%20Off))
  (bind _outactors (Actor|GetAllActorswithInterface "/Game/Blueprint/Nave/BPI_NaveStatus.BPI_NaveStatus_C"))
  (Class|BPINaveStatus|AddEnergyReducer(Message) _outactors (Variables|Default|GetEnergyCost)))

(event EventOn
  (Rendering|Material|SetMaterial (Variables|Default|GetSM_Lamp04) 0 (Variables|Default|GetMaterial%20On))
  (bind _outactors (Actor|GetAllActorswithInterface "/Game/Blueprint/Nave/BPI_NaveStatus.BPI_NaveStatus_C"))
  (Class|BPINaveStatus|RemoveEnergyReducer(Message) _outactors (Variables|Default|GetEnergyCost)))

(fn ConstructionScript
  (CallFunction|On))