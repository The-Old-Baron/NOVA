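; BP_Lamp01 is a lamp that switches on and off and wears down while lit.
; On applies the current state's material and plays a timeline whose event randomly lowers durability, deriving Normal, Danificado (damaged) or Quebrado (broken) unless Warning is set.
; That event then always applies the Normal material, and Quebrado has no material case.
; Off, also run at construction, sets the off material and stops the timeline.
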(event EventOff
  (Rendering|Material|SetMaterial (Variables|Default|GetSM_Lamp02) 0 (Variables|Default|GetMaterial%20Off))
  (Timeline|Timeline Stop
    (:Event
      (bind _output_get (Variables|Default|SetDurabilidade (- (Variables|Default|GetDurabilidade) (Math|Random|RandomFloatinRange 0.1 0.5))))
      (if (Utilities|Enum|Equal(Enum) (Variables|Default|GetEstado) "NewEnumerator3")
        _
        (elif (Math|Float|InRange(Float) _output_get 6e+01 1e+02)
          (Variables|Default|SetEstado "NewEnumerator0")
          (elif (Math|Float|InRange(Float) _output_get 1e+01 6e+01)
            (Variables|Default|SetEstado "NewEnumerator1")
            (else
              (Variables|Default|SetEstado "NewEnumerator2")))))
      (CallFunction|ApplyState "NewEnumerator0"))))

(event EventOn
  (CallFunction|ApplyState (Variables|Default|GetEstado))
  (Timeline|Timeline Play
    (:Event
      (bind _output_get (Variables|Default|SetDurabilidade (- (Variables|Default|GetDurabilidade) (Math|Random|RandomFloatinRange 0.1 0.5))))
      (if (Utilities|Enum|Equal(Enum) (Variables|Default|GetEstado) "NewEnumerator3")
        _
        (elif (Math|Float|InRange(Float) _output_get 6e+01 1e+02)
          (Variables|Default|SetEstado "NewEnumerator0")
          (elif (Math|Float|InRange(Float) _output_get 1e+01 6e+01)
            (Variables|Default|SetEstado "NewEnumerator1")
            (else
              (Variables|Default|SetEstado "NewEnumerator2")))))
      (CallFunction|ApplyState "NewEnumerator0"))))

(fn ConstructionScript
  (CallFunction|Off))

(fn ApplyState
  (params (Estado :type E_EquipmentStatus%20Enum :default "NewEnumerator0"))
  (bind _sm_lamp02 (Variables|Default|GetSM_Lamp02))
  (switch Utilities|FlowControl|Switch|SwitchonE_EquipmentStatus Estado
    (:NewEnumerator0
      (Rendering|Material|SetMaterial _sm_lamp02 0 (Variables|Default|GetMaterial%20On)))
    (:NewEnumerator1
      (Rendering|Material|SetMaterial _sm_lamp02 0 (Variables|Default|GetMaterial_Damage)))
    (:NewEnumerator3
      (Rendering|Material|SetMaterial _sm_lamp02 0 (Variables|Default|GetMaterail_Warning)))))