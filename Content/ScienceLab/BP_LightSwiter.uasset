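; BP_LightSwiter is an interactable push-button light switch that toggles a tagged group of lamps.
; On BeginPlay it collects every BPI_Lamp actor carrying its Tag into the Lights array, which the construction script clears.
; Interactwith plays a Timeline that moves the button top, and its Button Press event track flips State, sending on or off messages to each light.
; The item and fracture getters return fixed or empty values.
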(event EventBeginPlay
  (bind _outactors (Actor|GetAllActorswithInterface "/Game/ScienceLab/Meshes/Rooms/Lamps/BPI_Lamp.BPI_Lamp_C"))
  (for _array_element _outactors
    (if (Actor|ActorHasTag _array_element (Variables|Default|GetTag))
      (Utilities|Array|Add (Variables|Default|GetLights) _array_element))))

(event EventInteractwith
  (bind _alpha (Timeline|Timeline PlayFromStart)
    (:Update
      (Transformation|SetRelativeLocation (Variables|Default|GetSM_Button_Top) (Math|Vector|Lerp(Vector) "0, 0, 0" "0.000000,0.000000,-5.000000" _alpha) false false))
    (:ButtonPress
      (if (Variables|Default|GetState)
        (CallFunction|LightSwitch false)
        (else
          (CallFunction|LightSwitch true))))))

(fn ConstructionScript
  (Utilities|Array|Clear (Variables|Default|GetLights)))

(fn LightSwitch
  (params (IsOn :type Boolean))
  (Variables|Default|SetState IsOn)
  (for _array_element (Variables|Default|GetLights)
    (if IsOn
      (Class|BPILamp|On(Message) _array_element)
      (else
        (Class|BPILamp|Off(Message) _array_element)))))

(fn GetFractureBool
  (return false))

(fn GetItemType
  (return "NewEnumerator0"))

(fn GetMesh
  (return 0))