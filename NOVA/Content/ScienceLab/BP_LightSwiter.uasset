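; Interactable push-button light switch that toggles a group of lamps on and off.
; On BeginPlay it caches every BPI_Lamp actor carrying its Tag, then sends them on or off interface messages when toggled.
; Interaction plays a timeline that moves the button top, with an event track flipping the stored State.
; Item and look-at getters return placeholder values, and an OnRep function writes an integer to a text render, separate from the switch logic.
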(event Custom|Turn%20off
  (CallFunction|LightSwitch false))

(event Custom|TurnOn
  (CallFunction|LightSwitch true))

(event EventBeginPlay
  (bind _outactors (Actor|GetAllActorswithInterface "/Game/ScienceLab/Meshes/Rooms/Lamps/BPI_Lamp.BPI_Lamp_C"))
  (for _array_element _outactors
    (if (Actor|ActorHasTag _array_element (Variables|Default|GetTag))
      (Utilities|Array|Add (Variables|Default|GetLights) _array_element))))

(event EventInteractwith
  (params (PlayerCharacter :type BPC%20Player%20Object%20Reference))
  (bind _alpha (Timeline|Timeline PlayFromStart)
    (:Update
      (Transformation|SetRelativeLocation (Variables|Default|GetSM_Button_Top) (Math|Vector|Lerp(Vector) "0, 0, 0" "0.000000,0.000000,-5.000000" _alpha) false false))
    (:ButtonPress
      (if (Variables|Default|GetState)
        (CallFunction|TurnOff)
        (else
          (CallFunction|Turnon))))))

(fn ConstructionScript
  (Utilities|Array|Clear (Variables|Default|GetLights)))

(fn LightSwitch
  (params (IsOn :type Boolean))
  (Variables|Default|SetState IsOn)
  (for _array_element (Variables|Default|GetLights)
    (if IsOn
      (Class|BPILamp|On(Message) _array_element)
      (else
        (Class|BPILamp|Off(Message) _array_element)))))

(fn GetFractureBool
  (return false))

(fn GetItemType
  (return "NewEnumerator0"))

(fn GetMesh
  (return 0))

(fn OnRepInteiro
  (Rendering|Components|TextRender|SetText (Variables|Default|GetTextRender) (Utilities|Text|ToText(Integer) (Variables|Default|Getinteiro))))

(fn Lookat
  (return ""))