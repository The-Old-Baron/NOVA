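; BP_Nave is the ship Blueprint that holds energy consumption, energy storage, oxygen pressure and oxygen storage values behind getters and setters.
; Energy storage and oxygen pressure setters ignore values above their maximum, while SetStorageOxigen compares against the current amount, so it cannot increase it.
; AddEnergyStorage and RemoveEnergyStorage only return clamped results without storing them, unlike the consumption add/remove functions.
; GetAllAmbient is an empty stub, and nothing runs on Tick.
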(event EventBeginPlay)

(event Collision|EventActorBeginOverlap
  (params (OtherActor :type Actor%20Object%20Reference)))

(event EventTick
  (params (DeltaSeconds :type Float%20%28single-precision%29)))

(event EventSetEnergyConsuption
  (params (Energy%20Consuption :type Float%20%28double-precision%29))
  (Variables|Default|SetCurrent%20Energy%20Consuption Energy%20Consuption))

(event EventSetEnergyStorage
  (params (New%20Energy%20Storage :type Float%20%28double-precision%29))
  (if (<= New%20Energy%20Storage (Variables|Default|GetMax%20Energy%20Storage))
    (Variables|Default|SetCurrent%20Energy%20Storage New%20Energy%20Storage)))

(fn ConstructionScript)

(fn AddEnergyConsuption
  (params (Value :type Float%20%28double-precision%29))
  (bind _output_get (Variables|Default|SetCurrent%20Energy%20Consuption (+ (Variables|Default|GetCurrent%20Energy%20Consuption) Value)))
  (return _output_get))

(fn AddEnergyStorage
  (params (Value :type Float%20%28double-precision%29))
  (bind _current_energy_storage (Variables|Default|GetCurrent%20Energy%20Storage))
  (bind _max_energy_storage (Variables|Default|GetMax%20Energy%20Storage))
  (bind _returnvalue (+ _current_energy_storage Value))
  (if (<= _returnvalue _max_energy_storage)
    (return _returnvalue)
    (else
      (return _max_energy_storage))))

(fn GetAllAmbient)

(fn GetEnergyConsuption
  (return (Variables|Default|GetCurrent%20Energy%20Consuption)))

(fn GetEnergyStorage
  (return (Variables|Default|GetCurrent%20Energy%20Storage)))

(fn GetPressionOxigen
  (return (Variables|Default|GetCurrent%20Oxigen%20Pression)))

(fn GetStorageOxigen
  (return (Variables|Default|GetCurrent%20Oxigen%20Storage)))

(fn RemoveEnergyConsuption
  (params (Value :type Float%20%28double-precision%29))
  (bind _output_get (Variables|Default|SetCurrent%20Energy%20Consuption (- (Variables|Default|GetCurrent%20Energy%20Consuption) Value)))
  (return _output_get))

(fn RemoveEnergyStorage
  (params (Value :type Float%20%28double-precision%29))
  (bind _current_energy_storage (Variables|Default|GetCurrent%20Energy%20Storage))
  (bind _returnvalue (- _current_energy_storage Value))
  (if (<= _returnvalue 0.0)
    (return 0.0)
    (else
      (return _returnvalue))))

(fn SetPressionOxigen
  (params (Pression :type Float%20%28double-precision%29))
  (if (<= Pression (Variables|Default|GetMax%20Oxigen%20Pression))
    (bind _output_get (Variables|Default|SetCurrent%20Oxigen%20Pression Pression))
    (return _output_get)))

(fn SetStorageOxigen
  (params (Value :type Float%20%28double-precision%29))
  (if (<= Value (Variables|Default|GetCurrent%20Oxigen%20Storage))
    (bind _output_get (Variables|Default|SetCurrent%20Oxigen%20Storage Value))
    (return _output_get)))