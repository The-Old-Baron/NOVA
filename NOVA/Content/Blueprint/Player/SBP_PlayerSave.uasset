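; SaveGame Blueprint that holds the list of locally saved player characters, each with a unique ID, name and map name.
; Helper functions add characters and use linear searches to check, fetch or delete them by name.
; UpdateInfoByUID targets entries by unique ID for updating and prints "Save Not Found" after the loop.
; SaveToSlot writes the object itself to the fixed "Void_LocalChars" slot.
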(fn AddNewCharacter
  (params (UniqueID :type Integer) (Name :type Text))
  (Utilities|Array|Add (Variables|Default|GetSavedCharacters) (Utilities|Struct|MakeS_SavedLocalPlayer UniqueID Name)))

(fn DoesNameExist
  (params (Name :type Text))
  (for _array_element (Variables|Default|GetSavedCharacters)
    (if (Utilities|Enum|Equal(Enum) (.Name (Utilities|Struct|BreakS_SavedLocalPlayer _array_element)) Name)
      (return true)))
  (return false))

(fn GetCharacterbyName
  (params (Name :type Text))
  (for _array_element (Variables|Default|GetSavedCharacters)
    (if (Utilities|Enum|Equal(Enum) (.Name (Utilities|Struct|BreakS_SavedLocalPlayer _array_element)) Name)
      (return true _array_element)))
  (return false ""))

(fn DeleteCharacterbyName
  (params (Name :type Text))
  (for (_array_element _array_index) (Variables|Default|GetSavedCharacters)
    (if (Utilities|Enum|Equal(Enum) (.Name (Utilities|Struct|BreakS_SavedLocalPlayer _array_element)) Name)
      (Utilities|Array|RemoveIndex (Variables|Default|GetSavedCharacters) _array_index)
      (return true)))
  (return false))

(fn SavetoSlot
  (SaveGame|SaveGametoSlot self "Void_LocalChars"))

(fn UpdateInfobyUID
  (params (UID :type Integer) (Save :type S%20Saved%20Local%20Player%20Structure))
  (for (_array_element _array_index) (Variables|Default|GetSavedCharacters)
    (if (== (.UniqueID (Utilities|Struct|BreakS_SavedLocalPlayer _array_element)) UID)
      (Utilities|Struct|SetmembersinS_SavedLocalPlayer (Utilities|Array|Get(acopy) (Variables|Default|GetSavedCharacters) _array_index))))
  (Development|PrintString 0 "Save Not Found"))