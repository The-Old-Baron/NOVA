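; BP_AmbienceChange is a two-sided trigger that switches the player's current ambience between a left and a right setting.
; It overrides the parent's left and right trigger events, calling the parent logic first.
; Each event then sets the player's ambience message to that side's tag, but only if it differs from the current one.
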(fn ConstructionScript
  (|CallParentFunction))

(fn TriggerEventLeft
  (params (Player :type Pawn%20Object%20Reference))
  (bind _leftambiencetag (Variables|Default|GetLeftAmbienceTag))
  (|CallParentFunction Player)
  (bind _currentambience (Class|BPIPlayer|GetCurrentPlayerAmbience(Message) Player))
  (if (not (== _currentambience _leftambiencetag))
    (Class|BPIPlayer|SetCurrentPlayerAmbience(Message) Player _leftambiencetag)))

(fn TriggerEventRight
  (params (Player :type Pawn%20Object%20Reference))
  (bind _rightambiencetag (Variables|Default|GetRightAmbienceTag))
  (|CallParentFunction Player)
  (bind _currentambience (Class|BPIPlayer|GetCurrentPlayerAmbience(Message) Player))
  (if (not (== _currentambience _rightambiencetag))
    (Class|BPIPlayer|SetCurrentPlayerAmbience(Message) Player _rightambiencetag)))