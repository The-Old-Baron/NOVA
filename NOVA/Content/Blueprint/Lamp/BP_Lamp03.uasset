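; BP_Lamp03 is a lamp Blueprint that shows its condition by swapping the first material slot on its SMLamp01 component.
; On and Off events set the lit or unlit material directly.
; SetState passes a state to ApplyState, which maps normal, damaged (Danificado) and warning to their materials, with normal sharing the On material.
; The construction script starts the lamp in the normal state.
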(event EventSetState
  (params (States :type E_EquipmentStatus%20Enum :default "NewEnumerator0"))
  (CallFunction|ApplyState States))

(event EventOff
  (Rendering|Material|SetMaterial (Variables|Default|GetSM_Lamp01) 0 (Variables|Default|GetMaterial_Off)))

(event EventOn
  (Rendering|Material|SetMaterial (Variables|Default|GetSM_Lamp01) 0 (Variables|Default|GetMaterial_On)))

(fn ConstructionScript
  (CallFunction|ApplyState "NewEnumerator0"))

(fn ApplyState
  (params (Estado :type E_EquipmentStatus%20Enum :default "NewEnumerator0"))
  (switch Utilities|FlowControl|Switch|SwitchonE_EquipmentStatus Estado
    (:NewEnumerator0
      (Rendering|Material|SetMaterial (Variables|Default|GetSM_Lamp01) 0 (Variables|Default|GetMaterial_On)))
    (:NewEnumerator1
      (Rendering|Material|SetMaterial (Variables|Default|GetSM_Lamp01) 0 (Variables|Default|GetMaterial_Damage)))
    (:NewEnumerator3
      (Rendering|Material|SetMaterial (Variables|Default|GetSM_Lamp01) 0 (Variables|Default|GetMaterail_Warning)))))